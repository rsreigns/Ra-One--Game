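; Gameplay ability for the G-One hero's jump, which plays a flip montage and launches the player.
; When a flip is warranted, it starts the montage and waits for the jump gameplay event, launching only if a downward trace finds floor within range.
; It ends when the montage finishes or is cut short, or immediately without a flip.
; On ending, it sets the hero's movement mode to Falling.
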(event `self.K2_ActivateAbility`
  (bind _returnvalue (`self.GetAvatarActorFromActorInfo`))
  (bind _returnvalue_2 (`Actor.K2_GetActorLocation` _returnvalue))
  (`self.InitiateThisAbility`)
  (if (`self.bShouldFlip`)
    (`AbilityTask_PlayMontageAndWait.CreatePlayMontageAndWaitProxy` "None" (`self.MontageToPlay`)
      (:`then`
        (`AbilityTask_WaitGameplayEvent.WaitGameplayEvent` (struct :`TagName` "Player.Event.Jump") null
          (:`EventReceived`
            (bind _outhit (`KismetSystemLibrary.LineTraceSingle` _returnvalue_2 (- _returnvalue_2 (* (`Actor.GetActorUpVector` _returnvalue) (`self.FloorCheckDistance`))) "TraceTypeQuery1"))
            (if (`GameplayStatics.BreakHitResult` _outhit)
              (`self.LaunchPlayer`)))))
      (:`OnCompleted`
        (`self.K2_EndAbility` :!label _label))
      (:`OnBlendOut`
        (goto _label))
      (:`OnInterrupted`
        (goto _label))
      (:`OnCancelled`
        (goto _label)))
    (else
      (goto _label))))

(event `self.K2_OnEndAbility`
  (params (bWasCancelled :type Boolean))
  (`CharacterMovementComponent.SetMovementMode` (`Character.CharacterMovement` (`self.GetHeroCharacterFromAI`)) "MOVE_Falling" 0))