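; GM_TestHISM is a test Blueprint, likely a game mode, for exercising pooled Hierarchical Instanced Static Mesh objects.
; Its BeginPlay is empty, and the test chain is disconnected, so it never runs.
; That chain takes an object from BP_HISMSpawner's pool, scales it and binds it to the spawner's HISM.
; It then adds an instance above the player and removes index 0, repeating the removal after a delay and printing instance counts.
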(event `self.ReceiveBeginPlay`)

(fn `UserConstructionScript`)