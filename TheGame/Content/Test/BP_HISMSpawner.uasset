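; Test spawner that combines an actor pool of BP_ObjectToSpawn with a hierarchical instanced static mesh.
; BeginPlay pre-spawns the pool at its own transform and enables input.
; Left click moves a pooled actor in front of the player and adds a small mesh instance there.
; Right click sphere-traces forward and casts the hit actor, but instance removal is disconnected and ReturnToPool is never called here.
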(event `self.ReceiveBeginPlay`
  (set `self.PoolTransform` (`self.GetTransform`))
  (for _ (range (+ (`self.MaxPoolSize`) 1))
    (bind _returnvalue (`|SpawnActorFromClass` "/Game/Test/BP_ObjectToSpawn.BP_ObjectToSpawn_C" (`self.PoolTransform`) "AlwaysSpawn" "MultiplyWithRoot" null null))
    (`KismetArrayLibrary.Array_Add` (`self.ObjectPool`) _returnvalue)
    (`self.EnableInput` (`GameplayStatics.GetPlayerController` 0))))

(event `Key|LeftMouseButton`
  (params (Key :type "Key Structure"))
  (bind _returnvalue (`GameplayStatics.GetPlayerCharacter` 0))
  (bind _returnvalue_2 (+ (`self.K2_GetActorLocation` _returnvalue) (* (`self.GetActorForwardVector` _returnvalue) 300.0)))
  (:`Pressed`
    (`self.GetPoolObject` (`KismetMathLibrary.MakeTransform` _returnvalue_2))
    (`InstancedStaticMeshComponent.AddInstance` (`self.HierarchicalInstancedStaticMesh`) (`KismetMathLibrary.MakeTransform` _returnvalue_2 (struct) (0.1 0.1 0.1)) true)))

(event `Key|RightMouseButton`
  (params (Key :type "Key Structure"))
  (bind _returnvalue (`GameplayStatics.GetPlayerCharacter` 0))
  (bind _returnvalue_2 (`SceneComponent.K2_GetComponentLocation` (`Actor.RootComponent` _returnvalue)))
  (:`Pressed`
    (bind _outhit (`KismetSystemLibrary.SphereTraceSingle` :`Start` _returnvalue_2 :`End` (+ _returnvalue_2 (* (`SceneComponent.GetForwardVector` (`Actor.RootComponent` _returnvalue)) 2000.0)) :`Radius` 20.0 :`TraceChannel` "TraceTypeQuery1" :`DrawDebugType` "ForDuration" :`DrawTime` 2.0))
    (bind (_bblockinghit _binitialoverlap _time _distance _location _impactpoint _normal _impactnormal _physmat _hitactor _hitcomponent) (`GameplayStatics.BreakHitResult` _outhit))
    (if _bblockinghit
      (bind _asbp_object_to_spawn (cast `/Game/Test/BP_ObjectToSpawn` _hitactor)))))

(fn `GetPoolObject`
  (params (FTrans :type "Transform Structure"))
  (returns (`Array Element` :type "/Game/Test/BP_ObjectToSpawn Object Reference"))
  (locals (Loc_PoolObj :type "/Game/Test/BP_ObjectToSpawn Object Reference"))
  (bind _objectpool (`self.ObjectPool`))
  (bind _output (`|GetArrayItem` _objectpool))
  (if (> (`KismetArrayLibrary.Array_Length` _objectpool) 0)
    (`self.K2_SetActorTransform` _output FTrans false true)
    (`KismetArrayLibrary.Array_Remove` (`self.ObjectPool`))
    (return _output)))

(fn `ReturnToPool`
  (params (InObj :type "/Game/Test/BP_ObjectToSpawn Object Reference"))
  (`/Engine/EditorBlueprintResources/StandardMacros.IsValid` InObj
    (:`Is Valid`
      (`KismetArrayLibrary.Array_Add` (`self.ObjectPool`) InObj)
      (`KismetSystemLibrary.PrintString` "returned to pool")
      (return))))

(fn `UserConstructionScript`)