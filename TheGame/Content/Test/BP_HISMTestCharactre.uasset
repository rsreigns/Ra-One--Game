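; A flying test character, apparently for exercising HISM (hierarchical instanced static mesh) instance removal.
; On BeginPlay it adds an Enhanced Input mapping and switches to Flying, with camera-relative movement, mouse look, and E/Q debug keys for up/down.
; Right-click sphere-traces from the camera; a hit BP_ObjectToSpawn has the instance at its stored index removed from its referenced HISM component, rather than using the hit item.
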(event Input|EnhancedActionEvents|EnhancedInputActionIA_Move
  (params (ActionValue :type Vector%202D%20Structure) (ElapsedSeconds :type Float%20%28double-precision%29) (TriggeredSeconds :type Float%20%28double-precision%29) (InputAction :type Input%20Action%20Object%20Reference :default "/Game/Ra-One_Reborn/Input/Actions/Default/IA_Move.IA_Move"))
  (bind _camera (Variables|Default|GetCamera))
  (Pawn|Input|AddMovementInput (Math|Vector|GetForwardVector _camera) (.y ActionValue) false)
  (Pawn|Input|AddMovementInput (Math|Vector|GetRightVector _camera) (.x ActionValue) false))

(event Input|EnhancedActionEvents|EnhancedInputActionIA_Look
  (params (ActionValue :type Vector%202D%20Structure) (ElapsedSeconds :type Float%20%28double-precision%29) (TriggeredSeconds :type Float%20%28double-precision%29) (InputAction :type Input%20Action%20Object%20Reference :default "/Game/Ra-One_Reborn/Input/Actions/Default/IA_Look.IA_Look"))
  (Pawn|Input|AddControllerPitchInput (.y ActionValue))
  (Pawn|Input|AddControllerYawInput (.x ActionValue)))

(event EventBeginPlay
  (bind _asplayer_controller (Utilities|Casting|CastToPlayerController (Pawn|GetController)))
  (Utilities|IsValid (PlayerController|LocalPlayerSubsystems|GetEnhancedInputLocalPlayerSubsystem _asplayer_controller)
    (:Is%20Valid
      (Input|AddMappingContext (PlayerController|LocalPlayerSubsystems|GetEnhancedInputLocalPlayerSubsystem _asplayer_controller) "/Game/Ra-One_Reborn/Input/Mappings/IMC_G-One.IMC_G-One" 0 "(bIgnoreAllPressedKeysUntilRelease=True,bForceImmediately=False,bNotifyUserSettings=False)")
      (Pawn|Components|CharacterMovement|SetMovementMode (Variables|Character|GetCharacterMovement) "MOVE_Flying" 0))))

(event Input|KeyboardEvents|DebugKeyQ
  (params (Key :type Key%20Structure :default "None") (ActionValue :type Input%20Action%20Value%20Structure))
  (:Pressed
    (Pawn|Input|AddMovementInput (* (Math|Vector|GetUpVector (Variables|Default|GetCamera)) -1.0) 1.0 false)))

(event Input|KeyboardEvents|DebugKeyE
  (params (Key :type Key%20Structure :default "None") (ActionValue :type Input%20Action%20Value%20Structure))
  (:Pressed
    (Pawn|Input|AddMovementInput (Math|Vector|GetUpVector (Variables|Default|GetCamera)) 1.0 false)))

(event Input|MouseEvents|RightMouseButton
  (params (Key :type Key%20Structure :default "None"))
  (bind _camera (Variables|Default|GetCamera))
  (bind _returnvalue (Transformation|GetWorldLocation _camera))
  (:Pressed
    (bind _outhit (Collision|SphereTraceByChannel _returnvalue (+ _returnvalue (* (Math|Vector|GetForwardVector _camera) 2e+03)) 2e+01 "TraceTypeQuery1" false 0 "ForDuration" true "(R=1.000000,G=0.000000,B=0.000000,A=1.000000)" "(R=0.000000,G=1.000000,B=0.000000,A=1.000000)" 2.0))
    (if (.bBlockingHit (Collision|BreakHitResult _outhit))
      (bind _asbp_object_to_spawn (Utilities|Casting|CastToBP_ObjectToSpawn (.HitActor (Collision|BreakHitResult _outhit))))
      (Class|InstancedStaticMeshComponent|RemoveInstance (Variables|/Game/Test/BP_ObjectToSpawn.BP_ObjectToSpawn_C|GetHISMComonent _asbp_object_to_spawn) (Variables|/Game/Test/BP_ObjectToSpawn.BP_ObjectToSpawn_C|GetInstanceIndex _asbp_object_to_spawn)))))

(fn ConstructionScript)